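; BP_Switch is a lever switch that turns the website event on a BP_Screen actor's widget on or off.
; On BeginPlay it starts a looping timer and caches the ScreenWidget from the first BP_Screen found in the level.
; Each timer tick polls the Handle's relative pitch, calling enable while it sits within the negative quarter-turn range and disable otherwise, on every check rather than only on changes.
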(event Custom|LeverRotation_Check
  (if (Math|Float|InRange(Float) (.pitch (.rotation (Transformation|GetRelativeTransform (Variables|Default|GetHandle)))) -9e+01 0.0)
    (Default|EnableWebsiteEvent (Variables|Default|GetBP%20Screen%20Widget))
    (else
      (Default|DisableWebsiteEvent (Variables|Default|GetBP%20Screen%20Widget)))))

(event EventBeginPlay
  (Utilities|Time|SetTimerbyEvent (delegate Custom|LeverRotation_Check) 0.05 true)
  (bind _returnvalue (Actor|GetActorOfClass "/Game/DesignTest/Blueprints/UI/BP_Screen.BP_Screen_C"))
  (Utilities|IsValid _returnvalue
    (:Is%20Valid
      (bind _asscreen_widget (Utilities|Casting|CastToScreenWidget (UserInterface|GetUserWidgetObject (Variables|/Game/DesignTest/Blueprints/UI/BP_Screen.BP_Screen_C|GetWidget _returnvalue))))
      (Variables|Default|SetBP%20Screen%20Widget _asscreen_widget))))

(fn ConstructionScript)